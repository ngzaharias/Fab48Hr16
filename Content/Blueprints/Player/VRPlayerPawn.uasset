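; VRPlayerPawn is the player's VR pawn, forwarding motion controller input to two hand child actors.
; On BeginPlay it sets the right VRPlayerHand's Index to 1.
; Trigger presses and releases send use begin and finish messages to the matching hand.
; Grip inputs set per-hand flags, and Tick reloads the current level by name while both are held.
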(event EventBeginPlay
  (bind _asvrplayer_hand (Utilities|Casting|CastToVRPlayerHand (Variables|/Script/Engine.ChildActorComponent|GetChildActor (Variables|Default|GetRightHand))))
  (Variables|/Game/Blueprints/Player/VRPlayerHand.VRPlayerHand_C|SetIndex _asvrplayer_hand 1))

(event EventTick
  (params (DeltaSeconds :type Float%20%28single-precision%29))
  (if (and (Variables|Default|GetbIsLeftGripActive) (Variables|Default|GetbIsRightGripActive))
    (bind _returnvalue (Game|GetCurrentLevelName true))
    (Game|OpenLevel(byName) (Utilities|String|StringToName _returnvalue))))

(event Input|ActionEvents|InputActionTriggerLeft
  (params (Key :type Key%20Structure :default "AnyKey"))
  (bind _lefthand (Variables|Default|GetLeftHand))
  (bind _childactor (Variables|/Script/Engine.ChildActorComponent|GetChildActor _lefthand))
  (:Pressed
    (Class|IUseable|OnUseTriggerBegin(Message) _childactor))
  (:Released
    (Class|IUseable|OnUseTriggerFinish(Message) _childactor)))

(event Input|ActionEvents|InputActionTriggerRight
  (params (Key :type Key%20Structure :default "AnyKey"))
  (bind _righthand (Variables|Default|GetRightHand))
  (bind _childactor (Variables|/Script/Engine.ChildActorComponent|GetChildActor _righthand))
  (:Pressed
    (Class|IUseable|OnUseTriggerBegin(Message) _childactor))
  (:Released
    (Class|IUseable|OnUseTriggerFinish(Message) _childactor)))

(event Input|ActionEvents|InputActionGripLeft
  (params (Key :type Key%20Structure :default "AnyKey"))
  (:Pressed
    (Variables|Default|SetbIsLeftGripActive true))
  (:Released
    (Variables|Default|SetbIsLeftGripActive false)))

(event Input|ActionEvents|InputActionGripRight
  (params (Key :type Key%20Structure :default "AnyKey"))
  (:Pressed
    (Variables|Default|SetbIsRightGripActive true))
  (:Released
    (Variables|Default|SetbIsRightGripActive false)))

(fn ConstructionScript)