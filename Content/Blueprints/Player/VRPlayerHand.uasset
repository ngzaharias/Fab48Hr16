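; VR player hand that lets the player grab and release objects with the use trigger.
; A collider tracks overlapping components whose actors implement GrabInterface as grab targets.
; Trigger press picks the closest target to the hand mesh, checks that its owner allows grabbing, then starts GrabComponent and plays per-hand force feedback chosen by index.
; Trigger release ends the grab; the per-tick grab hook is empty.
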(event EventTick
  (params (DeltaSeconds :type Float%20%28single-precision%29))
  (Utilities|FlowControl|Sequence
    (:then_0
      (CallFunction|OnGrabTick))))

(event OnComponentBeginOverlap(GrabCollider)
  (params (OverlappedComponent :type Primitive%20Component%20Object%20Reference) (OtherActor :type Actor%20Object%20Reference) (OtherComp :type Primitive%20Component%20Object%20Reference) (OtherBodyIndex :type Integer) (bFromSweep :type Boolean) (SweepResult :type Hit%20Result%20Structure%20%28by%20ref%29))
  ;[1 1 1] Targets
  (if (Utilities|DoesObjectImplementInterface OtherActor (Variables|Grab|GetGrabInterface))
    (Utilities|Array|AddUnique (Variables|Grab|GetGrabTargets) OtherComp)))

(event OnComponentEndOverlap(GrabCollider)
  (params (OverlappedComponent :type Primitive%20Component%20Object%20Reference) (OtherActor :type Actor%20Object%20Reference) (OtherComp :type Primitive%20Component%20Object%20Reference) (OtherBodyIndex :type Integer))
  ;[1 1 1] Targets
  (if (Utilities|DoesObjectImplementInterface OtherActor (Variables|Grab|GetGrabInterface))
    (Utilities|Array|RemoveItem (Variables|Grab|GetGrabTargets) OtherComp)))

(event Custom|OnGrabBegin
  ;[1 1 1] Begin
  (if (> (Utilities|Array|Length (Variables|Grab|GetGrabTargets)) 0)
    (bind _returnvalue (Class|VRUtilityLibrary|GetClosestPrimitive (Transformation|GetWorldLocation (Variables|Default|GetStaticMesh)) (Variables|Grab|GetGrabTargets)))
    (bind _isnotgrabbable (Class|IGrabbable|IsNotGrabbable(Message) (Components|GetOwner _returnvalue)))
    (if (not _isnotgrabbable)
      (Class|VRGrabComponent|GrabBegin (Variables|Default|GetGrabComponent) (Utilities|Struct|MakeGrabInfo (Components|GetOwner _returnvalue) _returnvalue))
      (bind _asforce_feedback_effect (Utilities|Casting|CastToForceFeedbackEffect (Utilities|SelectObject "/Game/ForceFeedback/PickupEffect.PickupEffect" "/Game/ForceFeedback/PickupEffectRight.PickupEffectRight" (== (Variables|Default|GetIndex) 0))))
      (Game|Feedback|ClientPlayForceFeedback (Game|GetPlayerController 0) _asforce_feedback_effect false "None"))))

(event Custom|OnGrabFinish
  ;[1 1 1] Finish
  (Class|VRGrabComponent|GrabFinish (Variables|Default|GetGrabComponent)))

(event Custom|OnGrabTick
  ;[1 1 1] Tick
)

(event EventOnUseTriggerBegin
  (CallFunction|OnGrabBegin))

(event EventOnUseTriggerFinish
  (CallFunction|OnGrabFinish))

(fn ConstructionScript)