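; Base actor for unlock triggers, holding shared state checks and no event logic of its own.
; IsReady passes while the trigger is enabled and not yet triggered, and IsValidClass requires an exact class match with ClassRequired unless that equals ClassNone.
; IsReadyAndValid combines both checks, while nothing here sets the triggered flag or performs an unlock.
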(event EventBeginPlay)

(event Collision|EventActorBeginOverlap
  (params (OtherActor :type Actor%20Object%20Reference)))

(event EventTick
  (params (DeltaSeconds :type Float%20%28single-precision%29)))

(fn ConstructionScript)

(fn IsTriggered
  (return (Variables|Default|GetbIsTriggered)))

(fn IsValidClass
  (params (Object :type Object%20Object%20Reference))
  (bind _classrequired (Variables|Default|GetClassRequired))
  (return (or (== (Utilities|GetClass Object) _classrequired) (== _classrequired (Variables|Default|GetClassNone)))))

(fn IsReady
  (return (and (Variables|Default|GetbIsEnabled) (not (Variables|Default|GetbIsTriggered)))))

(fn IsReadyandValid
  (params (Object :type Object%20Object%20Reference))
  (bind _isvalid (CallFunction|IsValidClass Object))
  (bind _isready (CallFunction|IsReady))
  (return (and _isready _isvalid)))