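; Base lock actor that unlocks its Door and drops its mesh into physics simulation.
; Tick steps through UnlockSequence as each entry triggers, then advances LockState once KeyInserts meets its requirement, unlocking past LockStateRequired.
; BaseKey overlaps on Centre count inserts, start a named-function timer, and unlock immediately if the sequence is finished.
; The construction script applies the configurable mesh and sets Centre to overlap LockChannel.
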(event OnComponentBeginOverlap(Centre)
  (params (OverlappedComponent :type Primitive%20Component%20Object%20Reference) (OtherActor :type Actor%20Object%20Reference) (OtherComp :type Primitive%20Component%20Object%20Reference) (OtherBodyIndex :type Integer) (bFromSweep :type Boolean) (SweepResult :type Hit%20Result%20Structure%20%28by%20ref%29))
  (Utilities|Casting|CastToBaseKey OtherActor)
  (CallFunction|KeyInsert)
  (bind _finishedsequence (CallFunction|HasFinishedSequence))
  (if _finishedsequence
    (CallFunction|Unlock)))

(event EventBeginPlay)

(event Collision|EventActorBeginOverlap
  (params (OtherActor :type Actor%20Object%20Reference)))

(event EventTick
  (params (DeltaSeconds :type Float%20%28single-precision%29))
  (bind _finishedsequence (CallFunction|HasFinishedSequence))
  (if _finishedsequence
    (bind _hasfinished (CallFunction|HasFinishedLockState (Variables|Default|GetLockState)))
    (if _hasfinished
      (CallFunction|AdvanceLockState))
    (else
      (bind _triggered (Default|IsTriggered (Utilities|Array|Get(acopy) (Variables|Lock|GetUnlockSequence) (Variables|Lock|GetUnlockSequenceIndex))))
      (if _triggered
        (bind _result (Math|Integer|IncrementInt (Variables|Lock|GetUnlockSequenceIndex))
          (:%20%20
            (Variables|Lock|SetUnlockSequenceIndex _result)
            (Development|PrintString "Hello")))))))

(fn ConstructionScript
  (Components|StaticMesh|SetStaticMesh (Variables|Default|GetStaticMesh) (Variables|Lock|GetLockMesh))
  (Collision|SetCollisionResponsetoChannel (Variables|Default|GetCentre) (Variables|Lock|GetLockChannel) "ECR_Overlap"))

(fn LockStateReset
  (Utilities|FlowControl|Sequence
    (:then_0
      (Variables|Default|SetKeyInserts 0))
    (:then_1
      (Variables|Default|SetLockState 0))))

(fn KeyInsert
  (Variables|Default|SetKeyInserts (+ (Variables|Default|GetKeyInserts) 1))
  (if (not (Utilities|Time|IsTimerActivebyHandle (Variables|Default|GetTimerHandle)))
    (bind _returnvalue (Utilities|Time|SetTimerbyFunctionName 0 (Variables|Default|GetTimerFunction) (Variables|Default|GetTimerLength)))
    (Variables|Default|SetTimerHandle _returnvalue)))

(fn Unlock
  (Class|ILockable|Unlock(Message) (Variables|Default|GetDoor))
  (Physics|SetSimulatePhysics (Variables|Default|GetStaticMesh) true))

(fn AdvanceLockState
  (bind _output_get (Variables|Default|SetLockState (+ (Variables|Default|GetLockState) 1)))
  (if (> _output_get (Variables|Default|GetLockStateRequired))
    (CallFunction|Unlock)))

(fn HasFinishedLockState
  (params (LockState :type Integer))
  (switch int LockState
    (:Default
      (return false))
    (:0
      (if (>= (Variables|Default|GetKeyInserts) (Variables|Default|GetKeyInsertsRequired))
        (return true)
        (else
          (return false))))))

(fn HasFinishedSequence
  (return (>= (Variables|Lock|GetUnlockSequenceIndex) (Utilities|Array|Length (Variables|Lock|GetUnlockSequence)))))