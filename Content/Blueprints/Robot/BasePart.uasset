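; BasePart is a robot part actor whose static mesh can be restored to its authored placement.
; The construction script caches the mesh's relative location and rotation, and BeginPlay sets the root component's active state from IsActive.
; ResetActor disables physics and collision, reattaches the mesh to the root, then teleports it to the cached relative transform.
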(event EventBeginPlay
  (Components|Activation|SetActive (Variables|Default|GetDefaultSceneRoot) (Variables|Default|GetbIsActive) false))

(fn ConstructionScript
  (bind _staticmesh (Variables|Default|GetStaticMesh))
  (bind _returnvalue (Transformation|GetRelativeTransform _staticmesh))
  (Variables|Default|SetRelativeLocation (.location _returnvalue))
  (Variables|Default|SetRelativeRotation (.rotation _returnvalue)))

(fn ResetActor
  (bind _staticmesh (Variables|Default|GetStaticMesh))
  (Utilities|FlowControl|Sequence
    (:then_0
      (Physics|SetSimulatePhysics _staticmesh false)
      (Collision|SetCollisionEnabled _staticmesh "NoCollision"))
    (:then_1
      (Transformation|AttachComponentToComponent (Variables|Default|GetStaticMesh) (Variables|Default|GetDefaultSceneRoot) "None" "SnapToTarget" "SnapToTarget" "KeepRelative" true))
    (:then_2
      (Transformation|SetRelativeLocationAndRotation (Variables|Default|GetStaticMesh) (Variables|Default|GetRelativeLocation) (Variables|Default|GetRelativeRotation) false true))))