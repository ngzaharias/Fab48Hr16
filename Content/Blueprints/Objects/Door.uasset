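; Door actor that can be locked or unlocked, using physics simulation to open and color to show its state.
; BeginPlay creates a dynamic material instance from the door mesh's first material.
; Every Tick sets physics simulation on only while unlocked and tints the material red when locked or green when unlocked.
; An Unlock event clears the Locked flag.
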(event EventTick
  (params (DeltaSeconds :type Float%20%28single-precision%29))
  ;[1 1 1] Set physics and material color
  (Physics|SetSimulatePhysics (Variables|Default|GetDoor) (not (Variables|Default|GetLocked)))
  (Rendering|Material|SetVectorParameterValue (Variables|Default|GetMyMaterial) "Color" (select (Variables|Default|GetLocked) "(R=1.000000,G=0.000000,B=0.000000,A=1.000000)" "(R=0.000000,G=1.000000,B=0.000000,A=1.000000)") :!class /Script/Engine.MaterialInstanceDynamic))

(event EventUnlock
  ;[1 1 1] Setter for unlocking
  (Variables|Default|SetLocked false))

(event EventBeginPlay
  (bind _door (Variables|Default|GetDoor))
  ;[1 1 1] Clone material
  (bind _returnvalue (Rendering|Material|CreateDynamicMaterialInstance _door 0 (Rendering|Material|GetMaterial _door 0) :!class /Script/Engine.PrimitiveComponent))
  (Variables|Default|SetMyMaterial _returnvalue))

(fn ConstructionScript)